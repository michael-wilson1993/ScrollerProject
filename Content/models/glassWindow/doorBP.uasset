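; Window door actor that randomly swings open and shut once the side-scroller character has entered its trigger box.
; The box overlap sets a flag that is never cleared, which lets Tick run a delayed random roll repeatedly.
; On roughly half the rolls, the door rotates a quarter turn with sweep, then rotates back after a short random delay.
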(event `self.ReceiveTick`
  (params (DeltaSeconds :type "Float (single-precision)"))
  (bind _windowdoor (`self.windowDoor`))
  (if (`self.inoverlay`)
    (`KismetSystemLibrary.Delay` 2.0)
    (if (< (`KismetMathLibrary.RandomFloatInRange` 0.0 10.0) 5.0)
      (`SceneComponent.K2_AddLocalRotation` _windowdoor (struct :`Yaw` 90.0) true false)
      (`KismetSystemLibrary.Delay` (`KismetMathLibrary.RandomFloatInRange` 1.0 1.5))
      (`SceneComponent.K2_AddLocalRotation` _windowdoor (struct :`Yaw` -90.0) true false))))

(event `self.Box.OnComponentBeginOverlap`
  (params (OverlappedComponent :type "PrimitiveComponent Object Reference") (OtherActor :type "Actor Object Reference") (OtherComp :type "PrimitiveComponent Object Reference") (OtherBodyIndex :type Integer) (bFromSweep :type Boolean) (SweepResult :type "HitResult Structure (by ref)"))
  (cast `/Game/SideScrollerBP/Blueprints/SideScrollerCharacter` OtherActor)
  (set `self.inoverlay` true))

(fn `UserConstructionScript`)